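; Spline path Blueprint that continuously moves a referenced Actor, presumably a camera going by the asset name, along its spline.
; The construction script places that Actor at the first point, and a timeline, rate-scaled by TimelineLength, restarts whenever it finishes.
; Each update interpolates distance up to the last point and sets location from local-space spline coordinates.
; Rotation always follows the tangent at distance zero, not the current position.
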(event `self.ReceiveBeginPlay`
  (`TimelineComponent.SetPlayRate` (`self.时间轴`) (/ 1.0 (`self.TimelineLength`)))
  (`self.PlayTimeline`))

(event `PlayTimeline`
  (bind _spline (`self.Spline`))
  (bind _actor (`self.Actor`))
  (bind (_direction `_上下移动`) (`Timeline|时间轴` :!via `PlayFromStart`)
    (:`Update`
      (`self.K2_SetActorLocation` _actor (`SplineComponent.GetLocationAtDistanceAlongSpline` (`self.Spline`) (`KismetMathLibrary.Lerp` 0.0 (`SplineComponent.GetDistanceAlongSplineAtSplinePoint` _spline (- (`SplineComponent.GetNumberOfSplinePoints` _spline) 1)) `_上下移动`) "Local") false false)
      (`self.K2_SetActorRotation` _actor (`KismetMathLibrary.Conv_VectorToRotator` (`SplineComponent.GetTangentAtDistanceAlongSpline` (`self.Spline`) 0.0 "Local")) false))
    (:`Finished`
      (`self.PlayTimeline`))))

(fn `UserConstructionScript`
  (`self.K2_SetActorLocation` (`self.Actor`) (`SplineComponent.GetLocationAtSplinePoint` (`self.Spline`) 0 "Local") false false))