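; BP_Move_Trap is a spline-following trap that endlessly moves BPMovePlane from the first spline point to the last.
; BeginPlay scales the timeline's play rate by TimelineLength, and the timeline restarts itself whenever it finishes.
; Each update lerps distance along the spline, but applies local-space positions as world location and always takes rotation from the starting tangent.
; An unconnected world-space transform alternative remains in the graph.
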(event `self.ReceiveBeginPlay`
  (`TimelineComponent.SetPlayRate` (`self.Timeline`) (/ 1.0 (`self.TimelineLength`)))
  (`self.Play Timeline`))

(event `Play Timeline`
  (bind _spline (`self.Spline`))
  (bind _bp_moveplane (`self.BP_MovePlane`))
  (bind _spline_2 (`self.Spline`))
  (bind (_direction _newtrack_0) (`Timeline|Timeline` :!via `PlayFromStart`)
    (:`Update`
      (`SceneComponent.K2_SetWorldLocation` _bp_moveplane (`SplineComponent.GetLocationAtDistanceAlongSpline` _spline (`KismetMathLibrary.Lerp` 0.0 (`SplineComponent.GetDistanceAlongSplineAtSplinePoint` _spline_2 (- (`SplineComponent.GetNumberOfSplinePoints` _spline_2) 1)) _newtrack_0) "Local") false false)
      (`SceneComponent.K2_SetWorldRotation` _bp_moveplane (`KismetMathLibrary.Conv_VectorToRotator` (`SplineComponent.GetTangentAtDistanceAlongSpline` _spline 0.0 "Local")) false false))
    (:`Finished`
      (`self.Play Timeline`))))

(fn `UserConstructionScript`)