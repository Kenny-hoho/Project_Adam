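; Actor component that lets a Character grab, push and release pushable objects.
; BeginPush attaches the character to the object, disables orient-to-movement and enables tick; EndPush detaches and stops tick, leaving orient-to-movement off.
; Tick moves the object's static mesh along character forward/right vectors using move inputs and PushSpeed, but only within a limited yaw range.
; GetDeltaLocation also updates IsMovingAnObject, and debug logging remains throughout.
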(event `self.ReceiveBeginPlay`
  (`self.SetComponentTickEnabled` false)
  (bind _ascharacter (cast `Character` (`self.GetOwner`)))
  (set `self.Character` _ascharacter))

(event `self.ReceiveTick`
  (params (DeltaSeconds :type "Float (single-precision)"))
  (bind _forwardmove (`self.ForwardMove`))
  (bind _returnvalue (`self.GetDeltaLocation` DeltaSeconds _forwardmove (`self.RightMove`)))
  (bind (_returnvalue_roll _returnvalue_pitch _returnvalue_yaw) (`KismetMathLibrary.BreakRotator` (`Actor.K2_GetActorRotation` (`self.Character`))))
  (bind _output_get (set `self.CurrentActionRotation` _returnvalue_yaw))
  (if (`KismetMathLibrary.InRange_FloatFloat` _output_get 0.0 80.0)
    (`/Game/Pushable/BP_HelpLib.LogInfo` "To Right" (`KismetStringLibrary.Conv_DoubleToString` _output_get))
    (bind _currentpushableobject (`self.CurrentPushableObject`)
      (:`then`
        (`/Game/Pushable/BP_HelpLib.LogInfo` "delta" (`KismetStringLibrary.Conv_VectorToString` _returnvalue) true)
        (`/Game/Pushable/BP_HelpLib.LogInfo` "F:" (`KismetStringLibrary.Conv_DoubleToString` _forwardmove) true)
        (`SceneComponent.K2_AddWorldTransform` (`/Game/Pushable/BP_PushableObject.StaticMesh` _currentpushableobject) (`KismetMathLibrary.MakeTransform` _returnvalue) false false))
      (:`else`
        (`KismetSystemLibrary.PrintString` "Can Not Get Current PushableObject")))))

(fn `BeginPush`
  (params (PushObject :type "/Game/Pushable/BP_PushableObject Object Reference"))
  (bind _character (`self.Character`))
  (`KismetSystemLibrary.PrintString` "Begin Push")
  (`self.CurrentPushableObject`
    (:`then`)
    (:`else`
      (bind _output_get (set `self.CurrentPushableObject` PushObject))
      (`Actor.K2_AttachToActor` _character _output_get "None" "KeepWorld" "KeepWorld" "KeepWorld" true)
      (set `CharacterMovementComponent.bOrientRotationToMovement` false (`Character.CharacterMovement` _character))
      (`self.SetComponentTickEnabled` true))))

(fn `EndPush`
  (bind _character (`self.Character`))
  (`KismetSystemLibrary.PrintString` "End Push")
  (`self.CurrentPushableObject`
    (:`then`
      (set `self.CurrentPushableObject` null)
      (set `self.IsMovingAnObject` false)
      (`Actor.K2_DetachFromActor` _character "KeepWorld" "KeepWorld" "KeepWorld")
      (set `CharacterMovementComponent.bOrientRotationToMovement` false (`Character.CharacterMovement` _character))
      (`self.SetComponentTickEnabled` false))
    (:`else`)))

(fn `GetDeltaLocation`
  (params (DeltaSecond :type "Float (double-precision)") (ForwardMove :type "Float (double-precision)") (RightMove :type "Float (double-precision)"))
  (returns (ReturnValue :type "Vector Structure"))
  (set `self.IsMovingAnObject` (or (!= ForwardMove 0.0) (!= RightMove 0.0)))
  (return (+ (* (* (`Actor.GetActorForwardVector` (`self.Character`)) ForwardMove) (* (`self.PushSpeed`) DeltaSecond)) (* (* RightMove (`Actor.GetActorRightVector` (`self.Character`))) (* DeltaSecond (`self.PushSpeed`))))))

(fn `IsHoldingObject`
  (returns (Result :type Boolean))
  (return (`KismetSystemLibrary.IsValid` (`self.CurrentPushableObject`))))