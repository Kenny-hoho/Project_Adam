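; BP_DeadBody is a corpse actor that captures its skeletal pose and places a light at its location when none is already nearby.
; On BeginPlay it turns mesh physics simulation off, then after three seconds saves a "DeadPose" snapshot and enables actor collision.
; In parallel, after a short delay it spawns and configures a BP_Light if CreateLight is set.
; A Sphere overlap with another BP_Light clears that flag.
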(event `self.ReceiveBeginPlay`
  (`|ExecutionSequence`
    (:`then_0`
      (`PrimitiveComponent.SetSimulatePhysics` (`self.SkeletalMesh`) false)
      (`KismetSystemLibrary.Delay` 3.0)
      (`AnimInstance.SavePoseSnapshot` (`SkeletalMeshComponent.GetAnimInstance` (`self.SkeletalMesh`)) "DeadPose")
      (`PrimitiveComponent.SetSimulatePhysics` (`self.SkeletalMesh`) false)
      (`self.SetActorEnableCollision` true))
    (:`then_1`
      (`KismetSystemLibrary.Delay` 0.5)
      (if (`self.CreateLight`)
        (bind _returnvalue (`|SpawnActorFromClass` "/Game/MyActors/BP_Light.BP_Light_C" (`KismetMathLibrary.Conv_VectorToTransform` (`self.K2_GetActorLocation`)) "Undefined" "MultiplyWithRoot" null null))
        (bind _output_get (set `self.PointLigheRef` _returnvalue))
        (bind _pointlight (`/Game/MyActors/BP_Light.PointLight` _output_get))
        (`LightComponent.SetIntensity` _pointlight 200.0)
        (`LocalLightComponent.SetAttenuationRadius` _pointlight 3000.0)
        (`PointLightComponent.SetSourceRadius` _pointlight 1000.0)
        (else
          (`KismetSystemLibrary.PrintString` "NoNeed"))))))

(event `self.Sphere.OnComponentBeginOverlap`
  (params (OverlappedComponent :type "PrimitiveComponent Object Reference") (OtherActor :type "Actor Object Reference") (OtherComp :type "PrimitiveComponent Object Reference") (OtherBodyIndex :type Integer) (bFromSweep :type Boolean) (SweepResult :type "HitResult Structure (by ref)"))
  (cast `/Game/MyActors/BP_Light` OtherActor)
  (set `self.CreateLight` false)
  (`KismetSystemLibrary.PrintString` "AlreadyLight"))

(fn `UserConstructionScript`)