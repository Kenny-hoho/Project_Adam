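; A one-shot checkpoint actor that moves the player character to a new respawn point behind a screen fade.
; BeginPlay converts its respawn offset to a world location and takes the actor's rotation.
; When BP_AdamChar enters the box, it disables input, fades out and saves that transform as the RespawnPoint in BP_LevelGameMode.
; It then teleports the character there, fades in, restores input after CharacterFreezeTime and destroys itself.
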(event `SetRespawnPoint`
  ;[1 1 1] 设置gamemode里的复活点
  (bind _asbp_level_game_mode (cast `/Game/Levels/GameModes/BP_LevelGameMode` (`GameplayStatics.GetGameMode`)))
  (`KismetSystemLibrary.Delay` 0.2)
  (bind _output_get (set `/Game/Levels/GameModes/BP_LevelGameMode.RespawnPoint` (`KismetMathLibrary.MakeTransform` (`self.NextRespawnPoint`) (`self.NextRespawnRotation`)) _asbp_level_game_mode))
  (`KismetSystemLibrary.PrintString` (`KismetStringLibrary.Conv_TransformToString` _output_get)))

(event `self.ReceiveBeginPlay`
  ;[1 1 1] 初始化
  (set `self.NextRespawnRotation` (`self.K2_GetActorRotation`))
  (set `self.NextRespawnPoint` (+ (`self.K2_GetActorLocation`) (`self.NextRespawnPoint`))))

(event `self.Box.OnComponentBeginOverlap`
  (params (OverlappedComponent :type "PrimitiveComponent Object Reference") (OtherActor :type "Actor Object Reference") (OtherComp :type "PrimitiveComponent Object Reference") (OtherBodyIndex :type Integer) (bFromSweep :type Boolean) (SweepResult :type "HitResult Structure (by ref)"))
  (bind _asbp_adam_char (cast `/Game/Adam/Blueprint/BP_AdamChar` OtherActor))
  (bind _output_get (set `self.As BP Adam Char` _asbp_adam_char))
  (`self.DisableInput` _output_get (`GameplayStatics.GetPlayerController` 0))
  (`PlayerCameraManager.StartCameraFade` :`self` (`GameplayStatics.GetPlayerCameraManager` 0) :`ToAlpha` 1.0 :`Duration` 1.5 :`bHoldWhenFinished` true)
  (`self.SetRespawnPoint`)
  (`KismetSystemLibrary.Delay` 2.0)
  (`self.K2_TeleportTo` (`self.As BP Adam Char`) (`self.NextRespawnPoint`) (`self.NextRespawnRotation`))
  (`PlayerCameraManager.StartCameraFade` :`self` (`GameplayStatics.GetPlayerCameraManager` 0) :`FromAlpha` 1.0 :`Duration` 1.5 :`bHoldWhenFinished` true)
  (`KismetSystemLibrary.Delay` (`self.CharacterFreezeTime`))
  (`self.EnableInput` (`self.As BP Adam Char`) (`GameplayStatics.GetPlayerController` 0))
  (`self.K2_DestroyActor`))

(fn `UserConstructionScript`)