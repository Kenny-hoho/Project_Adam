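; BP_Movable is an object the player can drag while standing inside its Box trigger.
; Box overlap with BP_AdamChar enables and disables the actor's input.
; On Tick, holding Interact with nonzero Move X shifts it at the player's max speed, scaled by the world X component of the direction toward the player.
; The input's sign is only printed, so either direction pulls it toward the player.
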(event `self.ReceiveTick`
  (params (DeltaSeconds :type "Float (single-precision)"))
  (bind _returnvalue (`GameplayStatics.GetPlayerCharacter` 0))
  (bind _returnvalue_x (`KismetMathLibrary.BreakVector2D` (`|GetInputActionValue`)))
  (bind _staticmesh (`self.StaticMesh`))
  (if (`|GetInputActionValue`)
    (bind _returnvalue_2 (`HelpBlueprintBPLibrary.Sign` _returnvalue_x))
    (if _returnvalue_2
      (`KismetSystemLibrary.PrintText` (`KismetTextLibrary.Conv_BoolToText` _returnvalue_2))
      (`self.K2_SetActorTransform` (`KismetMathLibrary.MakeTransform` (+ (* (* (`GameplayStatics.GetWorldDeltaSeconds`) (`MovementComponent.GetMaxSpeed` (`Character.CharacterMovement` _returnvalue))) (* (`KismetMathLibrary.Vector_Forward`) (`KismetMathLibrary.Normal` (- (`self.K2_GetActorLocation` _returnvalue) (`SceneComponent.K2_GetComponentLocation` _staticmesh))))) (.location (`SceneComponent.K2_GetComponentToWorld` _staticmesh))) (.rotation (`SceneComponent.K2_GetComponentToWorld` _staticmesh)) (.scale (`SceneComponent.K2_GetComponentToWorld` _staticmesh)))))))

(event `self.Box.OnComponentBeginOverlap`
  (params (OverlappedComponent :type "PrimitiveComponent Object Reference") (OtherActor :type "Actor Object Reference") (OtherComp :type "PrimitiveComponent Object Reference") (OtherBodyIndex :type Integer) (bFromSweep :type Boolean) (SweepResult :type "HitResult Structure (by ref)"))
  (cast `/Game/Adam/BP_AdamChar` OtherActor)
  (`self.EnableInput` (`GameplayStatics.GetPlayerController` 0)))

(event `self.Box.OnComponentEndOverlap`
  (params (OverlappedComponent :type "PrimitiveComponent Object Reference") (OtherActor :type "Actor Object Reference") (OtherComp :type "PrimitiveComponent Object Reference") (OtherBodyIndex :type Integer))
  (cast `/Game/Adam/BP_AdamChar` OtherActor)
  (`self.DisableInput` (`GameplayStatics.GetPlayerController` 0)))

(fn `UserConstructionScript`)