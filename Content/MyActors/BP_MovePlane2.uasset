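; BP_MovePlane2 is a moving hazard that kills BP_AdamChar on contact and then displays its own corpse.
; A timeline, played from Tick, offsets the actor along local Z by MoveScale times MoveSpeed.
; Overlapping Box1 calls PlayerDied and turns off the character's CreateDeadBody flag.
; After a delay, it reveals the initially hidden DeadBody and enables collision on the separate Box component.
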(event `self.ReceiveBeginPlay`
  (`SceneComponent.SetVisibility` (`self.DeadBody`) false true)
  (`PrimitiveComponent.SetCollisionEnabled` (`self.Box`) "NoCollision"))

(event `self.ReceiveTick`
  (params (DeltaSeconds :type "Float (single-precision)"))
  (bind (_direction _movescale) (`Timeline|时间轴`)
    (:`Update`
      (`self.K2_AddActorLocalOffset` (`KismetMathLibrary.MakeVector` 0.0 0.0 (* _movescale (`self.MoveSpeed`)))))))

(event `self.Box1.OnComponentBeginOverlap`
  (params (OverlappedComponent :type "PrimitiveComponent Object Reference") (OtherActor :type "Actor Object Reference") (OtherComp :type "PrimitiveComponent Object Reference") (OtherBodyIndex :type Integer) (bFromSweep :type Boolean) (SweepResult :type "HitResult Structure (by ref)"))
  (bind _asbp_adam_char (cast `/Game/Adam/Blueprint/BP_AdamChar` OtherActor))
  (`/Game/Adam/Blueprint/BP_AdamChar.PlayerDied` _asbp_adam_char "S2D")
  (set `/Game/Adam/Blueprint/BP_AdamChar.CreateDeadBody` false _asbp_adam_char)
  (`KismetSystemLibrary.Delay` 2.0)
  (`SceneComponent.SetVisibility` (`self.DeadBody`) true true)
  (`PrimitiveComponent.SetCollisionEnabled` (`self.Box`) "QueryAndPhysics"))

(fn `UserConstructionScript`)