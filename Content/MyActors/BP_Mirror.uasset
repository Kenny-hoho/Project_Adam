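; BP_Mirror is an interactable mirror actor that opens the load-game menu for the player character.
; It creates a hidden W_LoadMenu widget on BeginPlay and uses a box trigger to bind or unbind OpenLoadWidget to BP_AdamChar's LoadGame event as the character enters or leaves.
; When that event fires, it shows the cursor, switches to UI-only input, pauses the game and reveals the menu.
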(event `self.ReceiveBeginPlay`
  (bind _returnvalue (`|CreateWidget` "/Game/UI/Widgets/W_LoadMenu.W_LoadMenu_C" null null))
  (bind _output_get (set `self.LoadMenuRef` _returnvalue))
  (`UserWidget.AddToViewport` _output_get 0)
  (`Widget.SetVisibility` (`self.LoadMenuRef`) "Collapsed"))

(event `self.Box.OnComponentBeginOverlap`
  (params (OverlappedComponent :type "PrimitiveComponent Object Reference") (OtherActor :type "Actor Object Reference") (OtherComp :type "PrimitiveComponent Object Reference") (OtherBodyIndex :type Integer) (bFromSweep :type Boolean) (SweepResult :type "HitResult Structure (by ref)"))
  (bind _asbp_adam_char (cast `/Game/Adam/BP_AdamChar` OtherActor))
  (add `/Game/Adam/BP_AdamChar.LoadGame` _asbp_adam_char (delegate `OpenLoadWidget`)))

(event `OpenLoadWidget`
  (bind _returnvalue (`GameplayStatics.GetPlayerController` 0))
  (set `PlayerController.bShowMouseCursor` true _returnvalue)
  (`WidgetBlueprintLibrary.SetInputMode_UIOnlyEx` _returnvalue null)
  (`GameplayStatics.SetGamePaused` true)
  (`Widget.SetVisibility` (`self.LoadMenuRef`) "Visible"))

(event `self.Box.OnComponentEndOverlap`
  (params (OverlappedComponent :type "PrimitiveComponent Object Reference") (OtherActor :type "Actor Object Reference") (OtherComp :type "PrimitiveComponent Object Reference") (OtherBodyIndex :type Integer))
  (bind _asbp_adam_char (cast `/Game/Adam/BP_AdamChar` OtherActor))
  (remove `/Game/Adam/BP_AdamChar.LoadGame` _asbp_adam_char (delegate `OpenLoadWidget`)))

(fn `UserConstructionScript`)