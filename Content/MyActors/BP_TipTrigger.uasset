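; BP_TipTrigger is a trigger actor that shows a W_Tip text widget in world space at an offset from itself.
; The tip is drawn when a BP_AdamChar overlaps its Box and no widget component is active, or at start if the BeginPlay flag is set.
; DrawTip creates the widget component at runtime, then TipFade fades and destroys it after Duration.
; In BeginPlay mode the actor also destroys itself afterwards.
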(event `self.ReceiveBeginPlay`
  (if (`self.BeginPlay`)
    (`self.DrawTip`)
    (`KismetSystemLibrary.Delay` (`self.Duration`))
    (`self.TipFade`)
    (`KismetSystemLibrary.Delay` 0.2)
    (`self.K2_DestroyActor`)))

(event `self.Box.OnComponentBeginOverlap`
  (params (OverlappedComponent :type "PrimitiveComponent Object Reference") (OtherActor :type "Actor Object Reference") (OtherComp :type "PrimitiveComponent Object Reference") (OtherBodyIndex :type Integer) (bFromSweep :type Boolean) (SweepResult :type "HitResult Structure (by ref)"))
  (cast `/Game/Adam/BP_AdamChar` OtherActor)
  (`/Engine/EditorBlueprintResources/StandardMacros.IsValid` (`self.WidgetComponentRef`)
    (:`Is Not Valid`
      (`self.DrawTip`))))

(event `DrawTip`
  (bind _widgetcomponentref (`self.WidgetComponentRef`))
  ;[1 1 1] 绘制提示
  (bind _returnvalue (`|CreateWidget` "/Game/UI/Widgets/W_Tip.W_Tip_C" null (`self.Tips`)))
  (set `self.TipWidgetRef` _returnvalue)
  (bind _returnvalue_2 (`AddComponent|NODE_AddWidgetComponent-1` :`RelativeTransform` (`self.WidgetOffset`)))
  (bind _output_get (set `self.WidgetComponentRef` _returnvalue_2))
  (`WidgetComponent.SetWidget` _output_get (`self.TipWidgetRef`))
  (`WidgetComponent.SetWidgetSpace` _widgetcomponentref "World")
  (`WidgetComponent.SetDrawAtDesiredSize` _widgetcomponentref true)
  (`KismetSystemLibrary.Delay` (`self.Duration`))
  (`self.TipFade`))

(event `TipFade`
  (`/Engine/EditorBlueprintResources/StandardMacros.IsValid` (`self.WidgetComponentRef`)
    (:`Is Valid`
      (`/Game/UI/Widgets/W_Tip.Fadeout` (`self.TipWidgetRef`))
      (`KismetSystemLibrary.Delay` 0.25)
      (`ActorComponent.K2_DestroyComponent` (`self.WidgetComponentRef`)))))

(fn `UserConstructionScript`)