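; BP_Hammer is a hammer trap that kills BP_AdamChar when it overlaps the trap's Box.
; On BeginPlay, event 111 plays a timeline that adds pitch rotation to the Hammer, and StaticMesh is hidden.
; An overlap calls PlayerDied, turns off the character's CreateDeadBody, and reveals StaticMesh after a short delay.
; A looping PlayTimeline variant that orbits the Hammer around Centre is left disconnected.
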(event `111`
  (bind (_direction _movescale) (`Timeline|时间轴`)
    (:`Update`
      (`SceneComponent.K2_AddWorldRotation` (`self.Hammer`) (`KismetMathLibrary.MakeRotator` 0.0 (* _movescale 0.5)) false false))))

(event `self.ReceiveBeginPlay`
  (`self.111`)
  (`SceneComponent.SetVisibility` (`self.StaticMesh`) false true))

(event `Play Timeline`
  (bind _hammer (`self.Hammer`))
  (bind _returnvalue (`SceneComponent.K2_GetComponentLocation` (`self.Centre`)))
  (bind (_direction _newtrack_0) (`Timeline|Timeline` :!via `PlayFromStart`)
    (:`Update`
      (bind _returnvalue_2 (`KismetMathLibrary.MakeRotator` 0.0 _newtrack_0))
      (`SceneComponent.K2_AddWorldRotation` _hammer _returnvalue_2 false false)
      (`SceneComponent.K2_SetWorldLocation` _hammer (+ _returnvalue (`KismetMathLibrary.GreaterGreater_VectorRotator` (- (`SceneComponent.K2_GetComponentLocation` _hammer) _returnvalue) _returnvalue_2)) false false))
    (:`Finished`
      (`self.Play Timeline`))))

(event `self.ReceiveTick`
  (params (DeltaSeconds :type "Float (single-precision)")))

(event `self.Box.OnComponentBeginOverlap`
  (params (OverlappedComponent :type "PrimitiveComponent Object Reference") (OtherActor :type "Actor Object Reference") (OtherComp :type "PrimitiveComponent Object Reference") (OtherBodyIndex :type Integer) (bFromSweep :type Boolean) (SweepResult :type "HitResult Structure (by ref)"))
  (bind _asbp_adam_char (cast `/Game/Adam/Blueprint/BP_AdamChar` OtherActor))
  (`/Game/Adam/Blueprint/BP_AdamChar.PlayerDied` _asbp_adam_char "S2D")
  (set `/Game/Adam/Blueprint/BP_AdamChar.CreateDeadBody` false _asbp_adam_char)
  (`KismetSystemLibrary.Delay` 2.0)
  (`SceneComponent.SetVisibility` (`self.StaticMesh`) true true))

(fn `RotateActorAroundThePoint`)

(fn `UserConstructionScript`)