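; BP_PushableTrap is a trap actor that kills BP_AdamChar on overlap, then becomes spent and shows its own dead body.
; BeginPlay configures its point light and either arms it with the body hidden or, without HasTrap, removes the trigger.
; Triggering suppresses the character's corpse creation, then reveals the trap's collidable body after delays and clears HasTrap.
; Every tick, a debug-drawn sphere trace along world +Y finds BP_Fog and destroys it once no trap remains.
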(event `self.ReceiveBeginPlay`
  (bind _pointlight (`self.PointLight`))
  (`parent.ReceiveBeginPlay`)
  (`LightComponent.SetIntensity` _pointlight (`self.LightIntensity`))
  (`LocalLightComponent.SetAttenuationRadius` _pointlight (`self.FadeRadius`))
  (`PointLightComponent.SetSourceRadius` _pointlight (`self.SourceRadius`))
  (if (`self.HasTrap`)
    (`SceneComponent.SetVisibility` (`self.DeadBody`) false true)
    (`PrimitiveComponent.SetCollisionEnabled` (`self.DeadBody`) "NoCollision")
    (set `self.AlreadyDead` false)
    (else
      (`ActorComponent.K2_DestroyComponent` (`self.TrapCollision`))
      (set `self.AlreadyDead` true))))

(event `self.TrapCollision.OnComponentBeginOverlap`
  (params (OverlappedComponent :type "PrimitiveComponent Object Reference") (OtherActor :type "Actor Object Reference") (OtherComp :type "PrimitiveComponent Object Reference") (OtherBodyIndex :type Integer) (bFromSweep :type Boolean) (SweepResult :type "HitResult Structure (by ref)"))
  (bind _asbp_adam_char (cast `/Game/Adam/Blueprint/BP_AdamChar` OtherActor))
  (bind _output_get (set `self.As BP Adam Char` _asbp_adam_char))
  (set `/Game/Adam/Blueprint/BP_AdamChar.CreateDeadBody` false _output_get)
  (`KismetSystemLibrary.Delay` 0.2)
  (`/Game/Adam/Blueprint/BP_AdamChar.PlayerDied` _output_get)
  (`ActorComponent.K2_DestroyComponent` (`self.TrapCollision`))
  (`KismetSystemLibrary.Delay` 2.0)
  (`SceneComponent.SetVisibility` (`self.DeadBody`) true true)
  (`PrimitiveComponent.SetCollisionEnabled` (`self.DeadBody`) "QueryAndPhysics")
  (set `self.AlreadyDead` true)
  (set `self.HasTrap` false))

(event `CheckFog`
  (bind _returnvalue (`self.K2_GetActorLocation`))
  (bind _outhit (`KismetSystemLibrary.SphereTraceSingle` :`Start` _returnvalue :`End` (+ _returnvalue (0.0 2000.0 0.0)) :`Radius` 50.0 :`TraceChannel` "TraceTypeQuery1" :`DrawDebugType` "ForOneFrame"))
  (bind _asbp_fog (cast `/Game/MyActors/BP_Fog` (`.HitActor` (`GameplayStatics.BreakHitResult` _outhit))))
  (set `self.RelativeFog` _asbp_fog)
  (if (not (`self.HasTrap`))
    (`/Game/MyActors/BP_Fog.DestroyFog` (`self.RelativeFog`))))

(event `self.ReceiveTick`
  (params (DeltaSeconds :type "Float (single-precision)"))
  (`self.CheckFog`))

(fn `UserConstructionScript`
  (`parent.UserConstructionScript`))