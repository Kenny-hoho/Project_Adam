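; BP_Door is a locked door that the player character BP_AdamChar opens with a matching key.
; Its Box overlap binds Open to the character's OpenDoor event on entry and unbinds it on exit, so only a nearby door responds.
; Open compares DoorIndex with the held key's MatchedDoorIndex, then calls DestroyItem on the character and plays a timeline that swings the mesh around yaw.
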(event `self.Box.OnComponentBeginOverlap`
  (params (OverlappedComponent :type "PrimitiveComponent Object Reference") (OtherActor :type "Actor Object Reference") (OtherComp :type "PrimitiveComponent Object Reference") (OtherBodyIndex :type Integer) (bFromSweep :type Boolean) (SweepResult :type "HitResult Structure (by ref)"))
  (bind _asbp_adam_char (cast `/Game/Adam/Blueprint/BP_AdamChar` OtherActor))
  (bind _output_get (set `self.AdamChar` _asbp_adam_char))
  (add `/Game/Adam/Blueprint/BP_AdamChar.OpenDoor` _output_get (delegate `Open`)))

(event `Open`
  (bind _keyref (`/Game/Adam/Blueprint/BP_AdamChar.KeyRef` (`self.AdamChar`)))
  (`/Engine/EditorBlueprintResources/StandardMacros.IsValid` _keyref
    (:`Is Valid`
      ;[1 1 1] 确认该钥匙是否能开此门
      (if (== (`self.DoorIndex`) (`/Game/MyActors/BP_Key.MatchedDoorIndex` _keyref))
        (`/Game/Adam/Blueprint/BP_AdamChar.DestroyItem` (`self.AdamChar`))
        (bind (_direction _rotateactor) (`Timeline|OpenDoorTimeline`)
          (:`Update`
            (`SceneComponent.K2_SetRelativeRotation` (`self.StaticMesh`) (`KismetMathLibrary.MakeRotator` 0.0 0.0 _rotateactor) false false)))))))

(event `self.Box.OnComponentEndOverlap`
  (params (OverlappedComponent :type "PrimitiveComponent Object Reference") (OtherActor :type "Actor Object Reference") (OtherComp :type "PrimitiveComponent Object Reference") (OtherBodyIndex :type Integer))
  (bind _asbp_adam_char (cast `/Game/Adam/Blueprint/BP_AdamChar` OtherActor))
  (remove `/Game/Adam/Blueprint/BP_AdamChar.OpenDoor` _asbp_adam_char (delegate `Open`)))

(fn `UserConstructionScript`)