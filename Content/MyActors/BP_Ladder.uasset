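; Ladder actor that lets BP_AdamChar start climbing down from the LadderDown trigger.
; Entering the trigger binds ClimbDown to the character's WantDown event; leaving clears all bindings on that event.
; ClimbDown teleports the character to ClimbDownStartPoint, with the ladder's rotation combined with a 180-degree turn.
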(event `self.LadderDown.OnComponentEndOverlap`
  (params (OverlappedComponent :type "PrimitiveComponent Object Reference") (OtherActor :type "Actor Object Reference") (OtherComp :type "PrimitiveComponent Object Reference") (OtherBodyIndex :type Integer))
  (bind _asbp_adam_char (cast `/Game/Adam/BP_AdamChar` OtherActor))
  (bind _output_get (set `self.AdamCharRef` _asbp_adam_char))
  (clear `/Game/Adam/BP_AdamChar.WantDown` _output_get))

(event `self.LadderDown.OnComponentBeginOverlap`
  (params (OverlappedComponent :type "PrimitiveComponent Object Reference") (OtherActor :type "Actor Object Reference") (OtherComp :type "PrimitiveComponent Object Reference") (OtherBodyIndex :type Integer) (bFromSweep :type Boolean) (SweepResult :type "HitResult Structure (by ref)"))
  (bind _asbp_adam_char (cast `/Game/Adam/BP_AdamChar` OtherActor))
  (bind _output_get (set `self.AdamCharRef` _asbp_adam_char))
  (add `/Game/Adam/BP_AdamChar.WantDown` _output_get (delegate `ClimbDown`)))

(event `ClimbDown`
  (`self.K2_SetActorLocationAndRotation` (`self.AdamCharRef`) (`SceneComponent.K2_GetComponentLocation` (`self.ClimbDownStartPoint`)) (`KismetMathLibrary.ComposeRotators` (`SceneComponent.K2_GetComponentRotation` (`self.Ladder`)) (struct :`Yaw` 180.0)) false false))

(fn `UserConstructionScript`)