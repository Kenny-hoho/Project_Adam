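; BP_DialogTrigger is a box trigger that lets BP_AdamChar open a dialog while standing inside it.
; Overlapping the box binds CreateDialog to the character's TriggerDialog event, and leaving unbinds it.
; CreateDialog shows the mouse cursor, switches to UI-only input and pauses the game.
; It then spawns either W_Dialog or W_TextBox, depending on WidgetClass, passing in DialogData and adding it to the viewport.
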(event `self.Box.OnComponentBeginOverlap`
  (params (OverlappedComponent :type "PrimitiveComponent Object Reference") (OtherActor :type "Actor Object Reference") (OtherComp :type "PrimitiveComponent Object Reference") (OtherBodyIndex :type Integer) (bFromSweep :type Boolean) (SweepResult :type "HitResult Structure (by ref)"))
  (bind _asbp_adam_char (cast `/Game/Adam/Blueprint/BP_AdamChar` OtherActor))
  (add `/Game/Adam/Blueprint/BP_AdamChar.TriggerDialog` _asbp_adam_char (delegate `CreateDialog`)))

(event `CreateDialog`
  (bind _returnvalue (`GameplayStatics.GetPlayerController` 0))
  (set `PlayerController.bShowMouseCursor` true _returnvalue)
  (`WidgetBlueprintLibrary.SetInputMode_UIOnlyEx` _returnvalue null)
  (`GameplayStatics.SetGamePaused` true)
  (bind _asw_dialog (castclass `/Game/UI/Widgets/W_Dialog` (`self.WidgetClass`))
    (:`then`
      (bind _returnvalue_2 (`|CreateWidget` _asw_dialog null (`self.DialogData`)))
      (`UserWidget.AddToViewport` _returnvalue_2 0))
    (:`CastFailed`
      (bind _asw_text_box (castclass `/Game/UI/Widgets/W_TextBox` (`self.WidgetClass`)))
      (bind _returnvalue_3 (`|CreateWidget` _asw_text_box null (`self.DialogData`)))
      (`UserWidget.AddToViewport` _returnvalue_3 0))))

(event `self.Box.OnComponentEndOverlap`
  (params (OverlappedComponent :type "PrimitiveComponent Object Reference") (OtherActor :type "Actor Object Reference") (OtherComp :type "PrimitiveComponent Object Reference") (OtherBodyIndex :type Integer))
  (bind _asbp_adam_char (cast `/Game/Adam/Blueprint/BP_AdamChar` OtherActor))
  (remove `/Game/Adam/Blueprint/BP_AdamChar.TriggerDialog` _asbp_adam_char (delegate `CreateDialog`)))

(fn `UserConstructionScript`)