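; Level game mode that sets up music, screen fade, respawn point and player state when a level starts.
; After a short delay on BeginPlay, it triggers BGM, defaults RespawnPoint to the PlayerStart and starts a camera fade.
; If BP_MyGameInstance flags a save load, it restores BP_AdamChar's location, death count and respawn point from SavedInfo.
; Otherwise, it copies only the death count from the GameInstance to the character.
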(event `self.ReceiveBeginPlay`
  (bind (_savedinfo_filename _savedinfo_levelname _savedinfo_location _savedinfo_deathnum _savedinfo_respawnpoint) (break `/Game/UI/Blueprints/SavedInfo` (`self.SavedInfo`)))
  (`KismetSystemLibrary.Delay` 1.0)
  (bind _returnvalue (`AddComponent|NODE_AddAudioComponent-0`))
  (`AudioParameterControllerInterface.SetTriggerParameter` _returnvalue "BGM")
  ;[1 1 1] 设置玩家复活点，默认为玩家出生点
  (bind _returnvalue_2 (`GameplayStatics.GetActorOfClass` "/Script/Engine.PlayerStart"))
  (set `self.RespawnPoint` (`self.GetTransform` _returnvalue_2))
  (`PlayerCameraManager.StartCameraFade` :`self` (`GameplayStatics.GetPlayerCameraManager` 0) :`FromAlpha` 1.0 :`Duration` (`self.Duration`) :`bHoldWhenFinished` true)
  (bind _asbp_my_game_instance (cast `/Game/Levels/GameModes/BP_MyGameInstance` (`GameplayStatics.GetGameInstance`)))
  (set `self.SavedInfo` (`/Game/Levels/GameModes/BP_MyGameInstance.SavedInfo` _asbp_my_game_instance))
  (if (`/Game/Levels/GameModes/BP_MyGameInstance.IsLoad` _asbp_my_game_instance)
    ;[1 1 1] 通过读取存档打开关卡时，将存档中的信息赋予玩家角色
    (bind _asbp_adam_char (cast `/Game/Adam/Blueprint/BP_AdamChar` (`GameplayStatics.GetPlayerCharacter` 0)))
    (`self.K2_SetActorLocation` _asbp_adam_char _savedinfo_location false false)
    (bind _output_get (set `/Game/Adam/Blueprint/BP_AdamChar.DeathNum` _savedinfo_deathnum _asbp_adam_char))
    (bind _asbp_my_game_instance_2 (cast `/Game/Levels/GameModes/BP_MyGameInstance` (`GameplayStatics.GetGameInstance`)))
    (set `/Game/Levels/GameModes/BP_MyGameInstance.DeathNum` _output_get _asbp_my_game_instance_2)
    (set `self.RespawnPoint` _savedinfo_respawnpoint)
    (`WidgetBlueprintLibrary.SetInputMode_GameOnly` (`GameplayStatics.GetPlayerController` 0))
    (else
      ;[1 1 1] 不是通过读档打开关卡时，从GameInstance中读取死亡次数并赋予玩家角色
      (bind _asbp_adam_char_2 (cast `/Game/Adam/Blueprint/BP_AdamChar` (`GameplayStatics.GetPlayerCharacter` 0)))
      (set `/Game/Adam/Blueprint/BP_AdamChar.DeathNum` (`/Game/Levels/GameModes/BP_MyGameInstance.DeathNum` _asbp_my_game_instance) _asbp_adam_char_2))))

(event `self.ReceiveTick`
  (params (DeltaSeconds :type "Float (single-precision)")))

(fn `UserConstructionScript`
  (`parent.UserConstructionScript`))